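; Player character for Adaptik, with camera-relative Enhanced Input movement, jumping, a HUD and a gravity-beam grab.
; A per-tick camera trace finds BPI_Fetchable objects, which a PhysicsHandle holds ahead of the camera until released or thrown, excluding whatever is underfoot.
; It supplies camera parameters with speed-based FOV and ignores look input during time dilation.
; Surface-aligned movement from three floor traces remains, but its Move call and timer are disconnected.
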(event `self.ReceiveBeginPlay`
  ;[1 1 1] Setup Input
  (bind _asplayer_controller (cast `PlayerController` (`self.GetController`)))
  (bind _output_get (set `self.PlayerController` _asplayer_controller))
  (bind _returnvalue (pcsubsystem `EnhancedInputLocalPlayerSubsystem` _output_get))
  (`/Engine/EditorBlueprintResources/StandardMacros.IsValid` _returnvalue
    (:`Is Valid`
      (`EnhancedInputSubsystemInterface.AddMappingContext` _returnvalue "/Game/Adaptik/Input/IMC_Adaptik.IMC_Adaptik" 0 (struct))
      (bind _asbp_camera_manager (cast `/Game/Adaptik/Blueprints/Camera/BP_CameraManager` (`GameplayStatics.GetPlayerCameraManager` 0)))
      (set `self.CameraManagerRef` _asbp_camera_manager)
      (bind _returnvalue_2 (`|CreateWidget` "/Game/Adaptik/Blueprints/UI/WBP_HUD.WBP_HUD_C" (`GameplayStatics.GetPlayerController` 0)))
      (`UserWidget.AddToViewport` _returnvalue_2 0))))

(event `MovementTick`
  (`self.MovementTrace`))

(event `EnhancedInput|/Game/Adaptik/Input/Actions/IA_Look`
  (params (ActionValue :type "Vector2D Structure") (ElapsedSeconds :type "Float (double-precision)") (TriggeredSeconds :type "Float (double-precision)") (InputAction :type "InputAction Object Reference" :default "/Game/Adaptik/Input/Actions/IA_Look.IA_Look"))
  ;[1 1 1] Handle Look
  (:`Triggered`
    (if (`KismetMathLibrary.NearlyEqual_FloatFloat` (`GameplayStatics.GetGlobalTimeDilation`) 1.0 0.01)
      (`|ExecutionSequence`
        (:`then_0`
          (`self.AddControllerPitchInput` ActionValue_Y))
        (:`then_1`
          (`self.AddControllerYawInput` ActionValue_X))))))

(event `EnhancedInput|/Game/Adaptik/Input/Actions/IA_Move`
  (params (ActionValue :type "Vector2D Structure") (ElapsedSeconds :type "Float (double-precision)") (TriggeredSeconds :type "Float (double-precision)") (InputAction :type "InputAction Object Reference" :default "/Game/Adaptik/Input/Actions/IA_Move.IA_Move"))
  (bind (_returnvalue_roll _returnvalue_pitch _returnvalue_yaw) (`KismetMathLibrary.BreakRotator` (`self.GetControlRotation`)))
  (bind (_returnvalue_roll_2 _returnvalue_pitch_2 _returnvalue_yaw_2) (`KismetMathLibrary.BreakRotator` (`self.GetControlRotation`)))
  (bind (_returnvalue_roll_3 _returnvalue_pitch_3 _returnvalue_yaw_3) (`KismetMathLibrary.BreakRotator` (`self.GetControlRotation`)))
  (bind (_returnvalue_x _returnvalue_y) (`KismetMathLibrary.BreakVector` (+ (* ActionValue_X (`KismetMathLibrary.GetRightVector` (`KismetMathLibrary.MakeRotator` _returnvalue_roll 0.0 _returnvalue_yaw))) (* ActionValue_Y (`KismetMathLibrary.GetForwardVector` (`KismetMathLibrary.MakeRotator` 0.0 0.0 _returnvalue_yaw_3))))))
  (:`Triggered`
    ;[1 1 1] Handle Move
    (`self.AddMovementInput` (`KismetMathLibrary.Normal` (`KismetMathLibrary.MakeVector` _returnvalue_x _returnvalue_y) 0.01))
    (set `self.LastMovementFrame` (`GameplayStatics.GetTimeSeconds`))
    (`self.K2_SetActorRotation` (`KismetMathLibrary.MakeRotator` 0.0 0.0 _returnvalue_yaw_2))))

(event `EnhancedInput|/Game/Adaptik/Input/Actions/IA_Jump`
  (params (ActionValue :type Boolean) (ElapsedSeconds :type "Float (double-precision)") (TriggeredSeconds :type "Float (double-precision)") (InputAction :type "InputAction Object Reference" :default "/Game/Adaptik/Input/Actions/IA_Jump.IA_Jump"))
  ;[1 1 1] HandleJump
  (:`Triggered`
    (`self.Jump`))
  (:`Completed`
    (`self.StopJumping`)))

(event `self.ReceiveTick`
  (params (DeltaSeconds :type "Float (single-precision)"))
  (bind _cameramanagerref (`self.CameraManagerRef`))
  ;[1 1 1] Tick
  (`|ExecutionSequence`
    (:`then_0`
      (`self.GrabTrace`)
      (if (`BlueprintGameplayTagLibrary.HasTag` (`self.GameplayTags`) (struct :`TagName` "Player.GrabbedObject"))
        (`PhysicsHandleComponent.SetTargetLocation` (`self.PhysicsHandle`) (+ (`/Game/Adaptik/Blueprints/Camera/BP_CameraManager.CameraLocation` _cameramanagerref) (+ (* (`SceneComponent.GetForwardVector` (`PlayerCameraManager.TransformComponent` _cameramanagerref)) (`self.GrabbedObjectDistance`)) (0.0 0.0 50.0))))))))

(event `EnhancedInput|/Game/Adaptik/Input/Actions/IA_Grab`
  (params (ActionValue :type Boolean) (ElapsedSeconds :type "Float (double-precision)") (TriggeredSeconds :type "Float (double-precision)") (InputAction :type "InputAction Object Reference" :default "/Game/Adaptik/Input/Actions/IA_Grab.IA_Grab"))
  (bind _gravbeam (`self.GravBeam`))
  (bind _gravbeamsfx (`self.GravBeamSFX`))
  (bind _cameramanagerref (`self.CameraManagerRef`))
  ;[1 1 1] Grab Event
  (:`Triggered`
    (`ActorComponent.Activate` _gravbeam false)
    (`NiagaraComponent.SetVariableVec3` _gravbeam "User.BeamEnd" (+ (`/Game/Adaptik/Blueprints/Camera/BP_CameraManager.CameraLocation` _cameramanagerref) (* (`SceneComponent.GetForwardVector` (`PlayerCameraManager.TransformComponent` _cameramanagerref)) (`self.TraceDistance`)))))
  (:`Started`
    (`self.GrabObject`)
    (`AudioComponent.Play` _gravbeamsfx 0.0))
  (:`Completed`
    (`self.ReleaseObject` false)
    (`ActorComponent.Deactivate` _gravbeam)
    (`AudioComponent.Stop` _gravbeamsfx)))

(event `EnhancedInput|/Game/Adaptik/Input/Actions/IA_Throw`
  (params (ActionValue :type Boolean) (ElapsedSeconds :type "Float (double-precision)") (TriggeredSeconds :type "Float (double-precision)") (InputAction :type "InputAction Object Reference" :default "/Game/Adaptik/Input/Actions/IA_Throw.IA_Throw"))
  ;[1 1 1] Release
  (:`Started`
    (`self.ReleaseObject` true)))

(event `Move`
  (bind _returnvalue (`self.K2_GetActorLocation`))
  (bind _targetlocation (`self.TargetLocation`))
  (if (> (+ (`KismetMathLibrary.Abs` (`self.GetInputAxisValue`)) (`KismetMathLibrary.Abs` (`self.GetInputAxisValue`))) 0.0)
    (if (> (`KismetMathLibrary.Vector_Distance` _targetlocation _returnvalue) 2.0)
      (`self.AddMovementInput` (`KismetMathLibrary.GetDirectionUnitVector` _returnvalue _targetlocation) 200.0)
      (`self.K2_SetActorRotation` (`KismetMathLibrary.RLerp` (`self.K2_GetActorRotation`) (`self.TargetRotation`) 0.01 true))
      (set `self.LastMovementFrame` (`GameplayStatics.GetTimeSeconds`)))))

(fn `GetCameraParameters`
  (returns (FOV :type "Float (double-precision)") (Offset :type "Vector Structure"))
  (return (+ (* (/ (`KismetMathLibrary.VSizeXY` (`self.GetVelocity`)) (`MovementComponent.GetMaxSpeed` (`self.CharacterMovement`))) 10.0) 90.0) (-300.0 50.0 50.0)))

(fn `GetMovementDirection`
  (returns (ReturnValue :type "Vector Structure"))
  (return (`KismetMathLibrary.Normal` (+ (* (`self.GetActorForwardVector`) (`self.GetInputAxisValue`)) (* (`self.GetActorRightVector`) (`self.GetInputAxisValue`))))))

(fn `GetViewSocket`
  (returns (Socket :type "Transform Structure"))
  (return (`KismetMathLibrary.MakeTransform` (`self.K2_GetActorLocation`))))

(fn `GrabObject`
  (bind (_out_hit_bblockinghit _out_hit_binitialoverlap _out_hit_time _out_hit_distance _out_hit_location _out_hit_impactpoint _out_hit_normal _out_hit_impactnormal _out_hit_physmat _out_hit_hitactor) (`GameplayStatics.BreakHitResult` (`self.Out Hit`)))
  (bind (_out_hit_bblockinghit_2 _out_hit_binitialoverlap_2 _out_hit_time_2 _out_hit_distance_2 _out_hit_location_2 _out_hit_impactpoint_2 _out_hit_normal_2 _out_hit_impactnormal_2 _out_hit_physmat_2 _out_hit_hitactor_2 _out_hit_hitcomponent) (`GameplayStatics.BreakHitResult` (`self.Out Hit`)))
  (if (and (`KismetSystemLibrary.IsValid` _out_hit_hitactor) (`KismetSystemLibrary.DoesImplementInterface` _out_hit_hitactor "/Game/Adaptik/Blueprints/Interfaces/BPI_Fetchable.BPI_Fetchable_C"))
    (bind _returnvalue (`self.CheckBelow` _out_hit_hitactor))
    (if _returnvalue
      (`PrimitiveComponent.SetUseCCD` _out_hit_hitcomponent true "None")
      (`PrimitiveComponent.SetMaterial` (`self.GetComponentByClass` _out_hit_hitactor_2 "/Script/Engine.StaticMeshComponent") 0 "/Game/Adaptik/Meshes/atlas-cube_Baked1.atlas-cube_Baked1")
      (`PhysicsHandleComponent.GrabComponentAtLocation` (`self.PhysicsHandle`) _out_hit_hitcomponent "None" (`SceneComponent.K2_GetComponentLocation` _out_hit_hitcomponent))
      (set `self.GrabbedActor` _out_hit_hitactor_2)
      (`BlueprintGameplayTagLibrary.AddGameplayTag` (`self.GameplayTags`) (struct :`TagName` "Player.GrabbedObject"))
      (return)
      (else
        (return)))))

(fn `GrabTrace`
  (bind _cameramanagerref (`self.CameraManagerRef`))
  (bind _cameralocation (`/Game/Adaptik/Blueprints/Camera/BP_CameraManager.CameraLocation` _cameramanagerref))
  (bind _outhit (`KismetSystemLibrary.LineTraceSingle` _cameralocation (+ _cameralocation (* (`SceneComponent.GetForwardVector` (`PlayerCameraManager.TransformComponent` _cameramanagerref)) (`self.TraceDistance`))) "TraceTypeQuery1"))
  (set `self.Out Hit` _outhit)
  (return))

(fn `MovementTrace`
  (locals (HitF1 :type "HitResult Structure") (HitF2 :type "HitResult Structure") (HitR :type "HitResult Structure"))
  (bind _returnvalue (`self.GetActorUpVector`))
  (bind _returnvalue_2 (`self.K2_GetActorLocation`))
  (bind _returnvalue_3 (`self.K2_GetActorLocation`))
  (bind _returnvalue_4 (`self.K2_GetActorLocation`))
  (bind _returnvalue_5 (`self.GetMovementDirection`))
  (bind (_hitf1_bblockinghit _hitf1_binitialoverlap _hitf1_time _hitf1_distance _hitf1_location _hitf1_impactpoint _hitf1_normal) (`GameplayStatics.BreakHitResult` (`local.HitF1`)))
  (bind (_hitf2_bblockinghit _hitf2_binitialoverlap _hitf2_time _hitf2_distance _hitf2_location) (`GameplayStatics.BreakHitResult` (`local.HitF2`)))
  (bind (_hitr_bblockinghit _hitr_binitialoverlap _hitr_time _hitr_distance _hitr_location) (`GameplayStatics.BreakHitResult` (`local.HitR`)))
  (bind (_outhit _returnvalue_6) (`KismetSystemLibrary.LineTraceSingle` :`Start` _returnvalue_4 :`End` (+ _returnvalue_4 (* (`self.GetMovementDirection`) 1000.0) (* (`self.GetActorUpVector`) -800.0)) :`TraceChannel` "TraceTypeQuery1" :`DrawDebugType` "ForDuration"))
  (if _returnvalue_6
    (set `local.HitF1` _outhit)
    (bind (_outhit_2 _returnvalue_7) (`KismetSystemLibrary.LineTraceSingle` :`Start` _returnvalue_2 :`End` (+ _returnvalue_2 (* (`self.GetMovementDirection`) 1100.0) (* (`self.GetActorUpVector`) -500.0)) :`TraceChannel` "TraceTypeQuery1" :`DrawDebugType` "ForDuration"))
    (if _returnvalue_7
      (set `local.HitF2` _outhit_2)
      (bind (_outhit_3 _returnvalue_8) (`KismetSystemLibrary.LineTraceSingle` :`Start` _returnvalue_3 :`End` (+ _returnvalue_3 (* _returnvalue_5 1000.0) (* _returnvalue -800.0) (* (`KismetMathLibrary.RotateAngleAxis` _returnvalue_5 0.0 _returnvalue) 100.0)) :`TraceChannel` "TraceTypeQuery1" :`DrawDebugType` "ForDuration"))
      (if _returnvalue_8
        (set `local.HitR` _outhit_3)
        (set `self.TargetLocation` (+ _hitf1_location (* _hitf1_normal 60.0)))
        (set `self.TargetRotation` (`KismetMathLibrary.MakeRotationFromAxes` (`KismetMathLibrary.GetDirectionUnitVector` _hitf1_location _hitf2_location) (`KismetMathLibrary.GetDirectionUnitVector` _hitf1_location _hitr_location) _hitf1_normal))))))

(fn `ReleaseObject`
  (params (ThrowObject :type Boolean))
  (bind _gameplaytags (`self.GameplayTags`))
  (bind _returnvalue (`PhysicsHandleComponent.GetGrabbedComponent` (`self.PhysicsHandle`)))
  (if (`BlueprintGameplayTagLibrary.HasTag` _gameplaytags (struct :`TagName` "Player.GrabbedObject"))
    (`PrimitiveComponent.SetMaterial` (`self.GetComponentByClass` (`self.GrabbedActor`) "/Script/Engine.StaticMeshComponent") 0 null)
    (`/Engine/EditorBlueprintResources/StandardMacros.IsValid` _returnvalue
      (:`Is Valid`
        (`PrimitiveComponent.SetUseCCD` _returnvalue false "None")
        (`PhysicsHandleComponent.ReleaseComponent` (`self.PhysicsHandle`))
        (`BlueprintGameplayTagLibrary.RemoveGameplayTag` _gameplaytags (struct :`TagName` "Player.GrabbedObject"))
        (if (`local.ThrowObject`)
          (message `/Game/Adaptik/Blueprints/Interfaces/BPI_Fetchable.ThrowObject` (`self.GrabbedActor`)))
        (set `self.GrabbedActor` null)
        (return)))))

(fn `UserConstructionScript`)