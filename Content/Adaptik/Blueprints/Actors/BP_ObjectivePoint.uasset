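; BP_ObjectivePoint is a placeable trigger that shows an on-screen objective with an editable title and content.
; It creates a WBP_Objective widget on BeginPlay, then displays it once, either immediately if ShowInstantly is set or when the player overlaps ObjectiveBox, sized in the construction script.
; The widget slides in and reverses out after a delay.
; ObjectiveComplete is empty, and the "Objective Complete!" sequence is disconnected.
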(event `self.ReceiveBeginPlay`
  (bind _objectivewidgetref (`self.ObjectiveWidgetRef`))
  (bind _objectivewidgetref_2 (`self.ObjectiveWidgetRef`))
  (bind _objectiveslide (`/Game/Adaptik/Blueprints/UI/WBP_Objective.ObjectiveSlide` _objectivewidgetref_2))
  (bind _returnvalue (`|CreateWidget` "/Game/Adaptik/Blueprints/UI/WBP_Objective.WBP_Objective_C" null (`self.ObjectiveTitle`) (`self.ObjectiveContent`)))
  (set `self.ObjectiveWidgetRef` _returnvalue)
  (if (`self.ShowInstantly`)
    (`/Engine/EditorBlueprintResources/StandardMacros.DoOnce` false
      (:`Completed`
        (set `/Game/Adaptik/Blueprints/UI/WBP_Objective.ObjectiveTitleText` (`self.ObjectiveTitle`) _objectivewidgetref)
        (set `/Game/Adaptik/Blueprints/UI/WBP_Objective.ObjectiveContentText` (`self.ObjectiveContent`) _objectivewidgetref)
        (`TextBlock.SetColorAndOpacity` (`/Game/Adaptik/Blueprints/UI/WBP_Objective.ObjectiveText` _objectivewidgetref) (make `SlateColor` (make `LinearColor` 1.0)))
        (`UserWidget.AddToViewport` _objectivewidgetref_2 0)
        (`UserWidget.PlayAnimation` _objectivewidgetref_2 _objectiveslide 0.0 1 "Forward" 1.0 false)
        (`KismetSystemLibrary.Delay` 5.0)
        (`UserWidget.PlayAnimation` _objectivewidgetref_2 _objectiveslide 0.0 1 "Reverse" 1.0 false)))))

(event `self.ObjectiveBox.OnComponentBeginOverlap`
  (params (OverlappedComponent :type "PrimitiveComponent Object Reference") (OtherActor :type "Actor Object Reference") (OtherComp :type "PrimitiveComponent Object Reference") (OtherBodyIndex :type Integer) (bFromSweep :type Boolean) (SweepResult :type "HitResult Structure (by ref)"))
  (bind _objectivewidgetref (`self.ObjectiveWidgetRef`))
  (bind _objectivewidgetref_2 (`self.ObjectiveWidgetRef`))
  (bind _objectiveslide (`/Game/Adaptik/Blueprints/UI/WBP_Objective.ObjectiveSlide` _objectivewidgetref_2))
  (if (`self.ShowInstantly`)
    _
    (elif (== OtherActor (`GameplayStatics.GetPlayerCharacter` 0))
      (`/Engine/EditorBlueprintResources/StandardMacros.DoOnce` false
        (:`Completed`
          (set `/Game/Adaptik/Blueprints/UI/WBP_Objective.ObjectiveTitleText` (`self.ObjectiveTitle`) _objectivewidgetref)
          (set `/Game/Adaptik/Blueprints/UI/WBP_Objective.ObjectiveContentText` (`self.ObjectiveContent`) _objectivewidgetref)
          (`TextBlock.SetColorAndOpacity` (`/Game/Adaptik/Blueprints/UI/WBP_Objective.ObjectiveText` _objectivewidgetref) (make `SlateColor` (make `LinearColor` 1.0 0.0 1.0 1.0)))
          (`UserWidget.AddToViewport` _objectivewidgetref_2 0)
          (`UserWidget.PlayAnimation` _objectivewidgetref_2 _objectiveslide 0.0 1 "Forward" 1.0 false)
          (`KismetSystemLibrary.Delay` 5.0)
          (`UserWidget.PlayAnimation` _objectivewidgetref_2 _objectiveslide 0.0 1 "Reverse" 1.0 false))))))

(event `ObjectiveComplete`)

(fn `UserConstructionScript`
  (`BoxComponent.SetBoxExtent` (`self.ObjectiveBox`) (`self.ObjectiveBoxSize`) true))